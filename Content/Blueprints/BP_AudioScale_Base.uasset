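; Base Blueprint for audio-reactive scale objects, providing shared helpers that read loudness analysis from the level's BP_AudioManager.
; InitAudioScale caches the actor's starting scale and finds the manager.
; Getters return the analyzed sound's duration and the normalized loudness for a channel at a given time from its LoudnessAnalyzer.
; SmoothData squares a value and remaps it to a clamped multiplier range; no graph here applies the scale.
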(fn ConstructionScript)

(fn InitAudioScale
  (bind _returnvalue (Transformation|GetActorScale3D))
  (Variables|Default|SetScaleX (.x _returnvalue))
  (Variables|Default|SetScaleY (.y _returnvalue))
  (Variables|Default|SetScaleZ (.z _returnvalue))
  (bind _returnvalue_2 (Actor|GetActorOfClass "/Game/Blueprints/BP_AudioManager.BP_AudioManager_C"))
  (Variables|Default|SetAudioManager _returnvalue_2))

(fn SmoothData
  (params (DataValue :type Float%20%28double-precision%29))
  (return (Math|Float|MapRangeClamped (Math|Float|Square DataValue) 0.0 1.0 1.0 2.0)))

(fn GetAudioDuration
  (return (Variables|/Script/Engine.SoundBase|GetDuration (Variables|/Script/AudioAnalyzer.AudioAnalyzerNRT|GetSound (Variables|/Game/Blueprints/BP_AudioManager.BP_AudioManager_C|GetLoudnessAnalyzer (Variables|Default|GetAudioManager))))))

(fn GetAnalyzedLoudness
  (params (AtTime :type Float%20%28double-precision%29))
  (return (Class|LoudnessNRT|GetNormalizedChannelLoudnessatTime (Variables|/Game/Blueprints/BP_AudioManager.BP_AudioManager_C|GetLoudnessAnalyzer (Variables|Default|GetAudioManager)) AtTime (Variables|Default|GetChannelIndex))))