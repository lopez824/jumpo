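; Audio-reactive shape actor that scales its Sphere component with the loudness of the playing audio.
; On BeginPlay it initializes audio scaling and binds to the AudioManager's MetaAudio playback-percent event.
; Each callback converts playback percent to time, samples analyzed loudness there, smooths it, then multiplies by ScaleVariance and per-axis scale factors to set the sphere's relative scale.
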(event Custom|OnAudioTick
  (params (PlayingSoundWave :type Sound%20Wave%20Object%20Reference) (PlaybackPercent :type Float%20%28single-precision%29))
  (bind _output_get (Variables|Default|SetPlaybackTime (* PlaybackPercent (CallFunction|GetAudioDuration))))
  (Transformation|SetRelativeScale3D (Variables|Default|GetSphere) (Math|Vector|MakeVector (* (CallFunction|SmoothData (CallFunction|GetAnalyzedLoudness _output_get)) (Variables|Default|GetScaleVariance) (Variables|Default|GetScaleX)) (* (CallFunction|SmoothData (CallFunction|GetAnalyzedLoudness _output_get)) (Variables|Default|GetScaleVariance) (Variables|Default|GetScaleY)) (* (CallFunction|SmoothData (CallFunction|GetAnalyzedLoudness _output_get)) (Variables|Default|GetScaleVariance) (Variables|Default|GetScaleZ)))))

(event EventBeginPlay
  (CallFunction|InitAudioScale)
  (EventDispatchers|BindEventtoOnAudioPlaybackPercent (Variables|/Game/Blueprints/BP_AudioManager.BP_AudioManager_C|GetMetaAudio (Variables|Default|GetAudioManager)) (delegate Custom|OnAudioTick)))

(fn ConstructionScript
  (|CallParentFunction))