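; BP_AudioManager is a music player that switches between four songs on key input and shows the current song's name, game and composer on a HUD.
; On BeginPlay it creates the HUD and plays the current LoudnessAnalyzer's sound on the MetaAudio component after a short delay.
; Each song input fades out, swaps in that index's analyzer from the Analyzers array, fades in its sound and updates the HUD.
; A separate input quits the game.
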(event Input|EnhancedActionEvents|EnhancedInputActionIA_Quit
  (params (ActionValue :type Boolean) (ElapsedSeconds :type Float%20%28double-precision%29) (TriggeredSeconds :type Float%20%28double-precision%29) (InputAction :type Input%20Action%20Object%20Reference :default "/Game/Input/Actions/IA_Quit.IA_Quit"))
  (:Triggered
    (Game|QuitGame 0 "Quit" false)))

(event Input|EnhancedActionEvents|EnhancedInputActionSong_1
  (params (ActionValue :type Boolean) (ElapsedSeconds :type Float%20%28double-precision%29) (TriggeredSeconds :type Float%20%28double-precision%29) (InputAction :type Input%20Action%20Object%20Reference :default "/Game/Input/Actions/Song_1.Song_1"))
  (:Triggered
    (CallFunction|PlaySongatIndex)))

(event Input|EnhancedActionEvents|EnhancedInputActionSong_2
  (params (ActionValue :type Boolean) (ElapsedSeconds :type Float%20%28double-precision%29) (TriggeredSeconds :type Float%20%28double-precision%29) (InputAction :type Input%20Action%20Object%20Reference :default "/Game/Input/Actions/Song_2.Song_2"))
  (:Triggered
    (CallFunction|PlaySongatIndex 1)))

(event Input|EnhancedActionEvents|EnhancedInputActionSong_3
  (params (ActionValue :type Boolean) (ElapsedSeconds :type Float%20%28double-precision%29) (TriggeredSeconds :type Float%20%28double-precision%29) (InputAction :type Input%20Action%20Object%20Reference :default "/Game/Input/Actions/Song_3.Song_3"))
  (:Triggered
    (CallFunction|PlaySongatIndex 2)))

(event Input|EnhancedActionEvents|EnhancedInputActionSong_4
  (params (ActionValue :type Boolean) (ElapsedSeconds :type Float%20%28double-precision%29) (TriggeredSeconds :type Float%20%28double-precision%29) (InputAction :type Input%20Action%20Object%20Reference :default "/Game/Input/Actions/Song_4.Song_4"))
  (:Triggered
    (CallFunction|PlaySongatIndex 3)))

(event EventBeginPlay
  (bind _returnvalue (UserInterface|CreateWidget "/Game/UI/UI_HUD.UI_HUD_C" (Game|GetPlayerController 0)))
  (bind _output_get (Variables|Default|SetHUD _returnvalue))
  (UserInterface|Viewport|AddtoViewport _output_get 0)
  (CallFunction|UpdateHUD)
  (Audio|Components|Audio|SetSound (Variables|Default|GetMetaAudio) (Variables|/Script/AudioAnalyzer.AudioAnalyzerNRT|GetSound (Variables|Default|GetLoudnessAnalyzer)))
  (Utilities|FlowControl|Delay 0.2)
  (Audio|Components|Audio|Play (Variables|Default|GetMetaAudio) 0.0))

(fn ConstructionScript)

(fn PlaySongatIndex
  (params (Index :type Integer))
  (bind _metaaudio (Variables|Default|GetMetaAudio))
  (Audio|Components|Audio|FadeOut (Variables|Default|GetMetaAudio) (Variables|Default|GetFadeDuration) 0.0 "Linear" :!class /Script/Engine.AudioComponent)
  (bind _output_get (Variables|Default|SetLoudnessAnalyzer (Utilities|Array|Get(acopy) (Variables|Default|GetAnalyzers) Index)))
  (Audio|Components|Audio|SetSound _metaaudio (Variables|/Script/AudioAnalyzer.AudioAnalyzerNRT|GetSound _output_get))
  (Audio|Components|Audio|FadeIn _metaaudio (Variables|Default|GetFadeDuration) 1.0 0.0 "Linear" :!class /Script/Engine.AudioComponent)
  (CallFunction|UpdateHUD Index))

(fn UpdateHUD
  (params (Index :type Integer))
  (bind _hud (Variables|Default|GetHUD))
  (bind _songdetails (Variables|Default|GetSongDetails))
  (bind _output (Utilities|Array|Get(acopy) _songdetails Index))
  (Rendering|Components|TextRender|SetText (Variables|/Game/UI/UI_HUD.UI_HUD_C|GetSongName _hud) (.name _output))
  (Rendering|Components|TextRender|SetText (Variables|/Game/UI/UI_HUD.UI_HUD_C|GetGameName _hud) (.game _output))
  (Rendering|Components|TextRender|SetText (Variables|/Game/UI/UI_HUD.UI_HUD_C|GetComposer _hud) (.composer _output)))